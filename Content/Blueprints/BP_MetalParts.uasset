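; BP_MetalParts is a metal part actor whose hot-metal material reflects a temperature that cools over time.
; On BeginPlay it creates a dynamic instance of MAT_HotMetal and assigns it to the first material slot of its StaticMesh.
; Each Tick lowers CurrentTemp by CoolingRate scaled by delta time, clamps it to a normalized range and writes it to the material's CurrentTemp parameter.
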(event `self.ReceiveBeginPlay`
  (`parent.ReceiveBeginPlay`)
  (bind _returnvalue (`KismetMaterialLibrary.CreateDynamicMaterialInstance` "/Game/Materials/MAT_HotMetal.MAT_HotMetal"))
  (bind _output_get (set `self.MaterialInstance` _returnvalue))
  (`PrimitiveComponent.SetMaterial` (`self.StaticMesh`) 0 _output_get))

(event `self.ReceiveTick`
  (params (DeltaSeconds :type "Float (single-precision)"))
  (`parent.ReceiveTick` DeltaSeconds)
  (bind _output_get (set `self.CurrentTemp` (`KismetMathLibrary.FClamp` (- (`self.CurrentTemp`) (* (`self.CoolingRate`) DeltaSeconds)))))
  (`MaterialInstanceDynamic.SetScalarParameterValue` (`self.MaterialInstance`) "CurrentTemp" _output_get))

(fn `UserConstructionScript`
  (`parent.UserConstructionScript`))