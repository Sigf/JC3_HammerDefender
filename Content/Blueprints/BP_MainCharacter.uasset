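; First-person player character that picks up, carries and throws physics objects and works crafting stations.
; A camera line trace each tick shows the targeted item's name on the crosshair widget.
; Action cycles furnace or workbench options, or grabs a pickable or freshly spawned object via PhysicsHandle, notifying its owning station.
; While carrying, holding Action charges a throw shown on a strength bar and releasing launches it; Throw launches at maximum strength.
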(event `self.ReceiveTick`
  (params (DeltaSeconds :type "Float (single-precision)"))
  (bind _returnvalue (`GameplayStatics.GetPlayerCameraManager` 0))
  (bind _returnvalue_2 (`PlayerCameraManager.GetCameraLocation` _returnvalue))
  (`|ExecutionSequence`
    (:`then_0`
      ;[1 1 1] Update Crosshair
      (bind _outhit (`KismetSystemLibrary.LineTraceSingle` _returnvalue_2 (+ _returnvalue_2 (* (`self.GetActorForwardVector` _returnvalue) (`self.GrabReach`))) "TraceTypeQuery1" true))
      (bind (_bblockinghit _binitialoverlap _time _distance _location _impactpoint _normal _impactnormal _physmat _hitactor) (`GameplayStatics.BreakHitResult` _outhit))
      (bind _output_get (set `self.SelectedObject` _hitactor))
      (set `self.SelectedSurfacePosition` _location)
      (if (`KismetSystemLibrary.DoesImplementInterface` _output_get "/Game/Blueprints/BPI_GetName.BPI_GetName_C")
        (bind _name (message `/Game/Blueprints/BPI_GetName.ShowName` _output_get))
        (`self.SetCrosshairText` _name)
        (else
          (`self.SetCrosshairText` ""))))
    (:`then_1`
      ;[1 1 1] Update Grab Target Locatin
      (if (`self.ObjectGrabbed`)
        (`PhysicsHandleComponent.SetTargetLocation` (`self.PhysicsHandle`) (+ (+ (`PlayerCameraManager.GetCameraLocation` (`GameplayStatics.GetPlayerCameraManager` 0)) (* (`KismetMathLibrary.GetForwardVector` (`self.GetControlRotation`)) (`self.itemDistance`))) (`self.GrabOffset`)))))
    (:`then_2`
      ;[1 1 1] Updates UI bar
      (if (`self.ActionPressed`)
        (if (not (`self.ObjectJustGrabbed`))
          (bind _output_get_2 (set `self.CurrentThrowStrength` (+ (`self.CurrentThrowStrength`) (* (`self.StrenghWindUpSpeed`) DeltaSeconds))))
          (set `/Game/Blueprints/UI/BP_Crosshair_Widget.CurrentStrength` _output_get_2 (`self.crosshair_widget`)))))))

(event `self.ReceiveBeginPlay`
  (bind _returnvalue (`|CreateWidget` "/Game/Blueprints/UI/BP_Crosshair_Widget.BP_Crosshair_Widget_C"))
  (bind _output_get (set `self.crosshair_widget` _returnvalue))
  (`UserWidget.AddToViewport` _output_get 0)
  (set `/Game/Blueprints/UI/BP_Crosshair_Widget.CurrentStrength` (`self.CurrentThrowStrength`) _output_get)
  (set `/Game/Blueprints/UI/BP_Crosshair_Widget.MaxStrength` (`self.ThrowMaxStrength`) _output_get)
  (`/Game/Blueprints/UI/BP_Crosshair_Widget.ToggleThrowStrengthBar` _output_get false))

(event `InputAxis|MoveForward`
  (params (AxisValue :type "Float (single-precision)"))
  (`self.AddMovementInput` (`KismetMathLibrary.Normal` (`KismetMathLibrary.MakeVector` (.x (`self.GetActorForwardVector`)) (.y (`self.GetActorForwardVector`)))) AxisValue))

(event `InputAxis|MoveRight`
  (params (AxisValue :type "Float (single-precision)"))
  (`self.AddMovementInput` (`self.GetActorRightVector`) AxisValue))

(event `InputAxis|Turn`
  (params (AxisValue :type "Float (single-precision)"))
  (`self.AddControllerYawInput` AxisValue))

(event `InputAxis|LookUp`
  (params (AxisValue :type "Float (single-precision)"))
  (`self.AddControllerPitchInput` AxisValue))

(event `InputAction|Jump`
  (params (Key :type "Key Structure"))
  (:`Pressed`
    (`self.Jump`)))

(event `InputAction|Action`
  (params (Key :type "Key Structure"))
  (bind _selectedobject (`self.SelectedObject`))
  (:`Pressed`
    (set `self.ActionPressed` true)
    (if (`self.ObjectGrabbed`)
      (`/Game/Blueprints/UI/BP_Crosshair_Widget.ToggleThrowStrengthBar` (`self.crosshair_widget`) true)
      (else
        (bind _asbp_furnace (cast `/Game/Blueprints/Stations/BP_Furnace` _selectedobject)
          (:`then`
            (`/Game/Blueprints/Stations/BP_Furnace.CircleCraftableObjects` _asbp_furnace))
          (:`CastFailed`
            (bind _asbp_woodworking_bench (cast `/Game/Blueprints/Stations/BP_WoodworkingBench` _selectedobject)
              (:`then`
                (`/Game/Blueprints/Stations/BP_WoodworkingBench.CycleOptions` _asbp_woodworking_bench))
              (:`CastFailed`
                (`self.PickUpObject`)
                (set `self.ObjectJustGrabbed` true))))))))
  (:`Released`
    (set `self.ActionPressed` false)
    (if (`self.ObjectJustGrabbed`)
      (set `self.ObjectJustGrabbed` false)
      (else
        (`/Engine/EditorBlueprintResources/StandardMacros.IsValid` (`self.EquippedObject`)
          (:`Is Valid`
            (`self.ThrowObject` (`self.CurrentThrowStrength`))
            (`/Game/Blueprints/UI/BP_Crosshair_Widget.ToggleThrowStrengthBar` (`self.crosshair_widget`) false)))))))

(event `InputAction|Throw`
  (params (Key :type "Key Structure"))
  (:`Pressed`
    (`/Engine/EditorBlueprintResources/StandardMacros.IsValid` (`self.EquippedObject`)
      (:`Is Valid`
        (`self.ThrowObject` (`self.ThrowMaxStrength`))))))

(fn `GrabObject`
  (params (ItemDistance :type "Float (double-precision)") (GrabbedLocation :type "Vector Structure") (NewObject :type "/Game/Blueprints/BaseClasses/BP_PickableObject Object Reference"))
  (set `self.itemDistance` ItemDistance)
  (bind _output_get (set `self.GrabbedLocatin` GrabbedLocation))
  (bind _output_get_2 (set `self.EquippedObject` NewObject))
  (bind _asbp_pickable_static (cast `/Game/Blueprints/BaseClasses/BP_PickableStatic` _output_get_2))
  (`PhysicsHandleComponent.GrabComponentAtLocation` (`self.PhysicsHandle`) (`/Game/Blueprints/BaseClasses/BP_PickableStatic.StaticMesh` _asbp_pickable_static) "None" _output_get)
  (set `self.ObjectGrabbed` true)
  (bind _stationowner (`/Game/Blueprints/BaseClasses/BP_PickableObject.StationOwner` _asbp_pickable_static))
  (if (`KismetSystemLibrary.DoesImplementInterface` _stationowner "/Game/Blueprints/BPI_DropObject.BPI_DropObject_C")
    (message `/Game/Blueprints/BPI_DropObject.DropObject` _stationowner NewObject)
    (set `/Game/Blueprints/BaseClasses/BP_PickableObject.StationOwner` self _asbp_pickable_static)))

(fn `PickUpObject`
  (bind _returnvalue (`GameplayStatics.GetPlayerCameraManager` 0))
  (bind _returnvalue_2 (`PlayerCameraManager.GetCameraLocation` _returnvalue))
  (bind _outhit (`KismetSystemLibrary.LineTraceSingle` _returnvalue_2 (+ _returnvalue_2 (* (`self.GetActorForwardVector` _returnvalue) (`self.GrabReach`))) "TraceTypeQuery1" true))
  (bind (_bblockinghit _binitialoverlap _time _distance _location _impactpoint _normal _impactnormal _physmat _hitactor) (`GameplayStatics.BreakHitResult` _outhit))
  (bind _asbp_pickable_object (cast `/Game/Blueprints/BaseClasses/BP_PickableObject` _hitactor)
    (:`then`
      (`self.GrabObject` _distance _location _asbp_pickable_object))
    (:`CastFailed`
      (bind _asbp_object_spawner (cast `/Game/Blueprints/BaseClasses/BP_ObjectSpawner` _hitactor))
      (bind _returnvalue_3 (`|SpawnActorFromClass` (`/Game/Blueprints/BaseClasses/BP_ObjectSpawner.ClassToSpawn` _asbp_object_spawner) (`KismetMathLibrary.MakeTransform` _location) "Undefined" "OverrideRootScale" null null))
      (`self.GrabObject` _distance _location _returnvalue_3))))

(fn `SetCrosshairText`
  (params (Text :type Text))
  (bind _crosshair_widget (`self.crosshair_widget`))
  (`/Engine/EditorBlueprintResources/StandardMacros.IsValid` _crosshair_widget
    (:`Is Valid`
      (`/Game/Blueprints/UI/BP_Crosshair_Widget.SetSelectedItem` _crosshair_widget Text))))

(fn `SetCrosshairTexture`
  (params (Texture :type "Texture2D Object Reference"))
  (bind _crosshair_widget (`self.crosshair_widget`))
  (`/Engine/EditorBlueprintResources/StandardMacros.IsValid` _crosshair_widget
    (:`Is Valid`
      (`/Game/Blueprints/UI/BP_Crosshair_Widget.SetCrosshairTexture` _crosshair_widget Texture))))

(fn `ThrowObject`
  (params (ThrowStrength :type "Float (double-precision)"))
  (if (`self.ObjectGrabbed`)
    (bind _asbp_pickable_static (cast `/Game/Blueprints/BaseClasses/BP_PickableStatic` (`self.EquippedObject`)))
    (`PhysicsHandleComponent.ReleaseComponent` (`self.PhysicsHandle`))
    (`PrimitiveComponent.AddImpulse` (`/Game/Blueprints/BaseClasses/BP_PickableStatic.StaticMesh` _asbp_pickable_static) (* (`KismetMathLibrary.GetForwardVector` (`self.GetControlRotation`)) ThrowStrength) "None" true)
    (set `self.ObjectGrabbed` false)
    (set `self.EquippedObject` null)
    (set `self.CurrentThrowStrength` 0.0)))

(fn `UnEquipObject`
  (set `self.EquippedObject` null)
  (set `self.ObjectGrabbed` false)
  (`PhysicsHandleComponent.ReleaseComponent` (`self.PhysicsHandle`)))

(fn `UserConstructionScript`)