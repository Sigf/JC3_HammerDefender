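; BP_CatcherObject is an actor that catches accepted BP_PickableObject classes entering its sphere, sized by CatchRadius in the construction script.
; On overlap it increments Count, destroys the object and fires ObjectCaught, first unequipping it from BP_MainCharacter if held.
; StoreObject routes through SlotObject, but both paths only keep a count.
; PopObject just decrements Count without spawning anything back.
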(event `self.Sphere.OnComponentBeginOverlap`
  (params (OverlappedComponent :type "PrimitiveComponent Object Reference") (OtherActor :type "Actor Object Reference") (OtherComp :type "PrimitiveComponent Object Reference") (OtherBodyIndex :type Integer) (bFromSweep :type Boolean) (SweepResult :type "HitResult Structure (by ref)"))
  (bind _asbp_pickable_object (cast `/Game/Blueprints/BP_PickableObject` OtherActor))
  (if (`KismetArrayLibrary.Array_Contains` (`self.AcceptingObjects`) (`GameplayStatics.GetObjectClass` _asbp_pickable_object))
    (if (`self.StoreObject`)
      (`self.SlotObject` _asbp_pickable_object)
      (`self.ObjectCaught`)
      (else
        (`/Engine/EditorBlueprintResources/StandardMacros.IncrementInt` (`self.Count`)
          (:`  `
            (`self.UnequipObject` _asbp_pickable_object)
            (`self.ObjectCaught`)))))))

(fn `PopObject`
  (bind _count (`self.Count`))
  (if (> _count 0)
    (`/Engine/EditorBlueprintResources/StandardMacros.DecrementInt` _count
      (:`  `
        _)))
  (return))

(fn `SlotObject`
  (params (NewObject :type "/Game/Blueprints/BP_PickableObject Object Reference"))
  (`self.UnequipObject` NewObject)
  (`/Engine/EditorBlueprintResources/StandardMacros.IncrementInt` (`self.Count`)
    (:`  `
      (`self.K2_DestroyActor` NewObject))))

(fn `UnequipObject`
  (params (Object :type "/Game/Blueprints/BP_PickableObject Object Reference"))
  (bind _asbp_main_character (cast `/Game/Blueprints/BP_MainCharacter` (`GameplayStatics.GetPlayerPawn` 0)))
  (if (== (`/Game/Blueprints/BP_MainCharacter.EquippedObject` _asbp_main_character) Object)
    (`/Game/Blueprints/BP_MainCharacter.UnEquipObject` _asbp_main_character)
    (`self.K2_DestroyActor` Object)
    (else
      (`self.K2_DestroyActor` Object)))
  (return))

(fn `UserConstructionScript`
  (`SphereComponent.SetSphereRadius` (`self.Sphere`) (`self.CatchRadius`) false))