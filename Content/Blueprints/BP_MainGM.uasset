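; BP_MainGM is the main game mode, running a timed round that ends in a level clear or failure based on score.
; StartTimer enables the countdown and broadcasts TimerStarted, then Tick accumulates elapsed time until it reaches the time limit.
; On expiry it stops counting, broadcasts TimerFinished, then compares Score to ScoreLimit to broadcast LevelCleared or LevelFailed.
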(event `self.ReceiveTick`
  (params (DeltaSeconds :type "Float (single-precision)"))
  (if (`self.CountDown`)
    (bind _output_get (set `self.ElapsedTime` (+ (`self.ElapsedTime`) DeltaSeconds)))
    (if (>= _output_get (`self.TimeLimit`))
      (set `self.CountDown` false)
      (`self.TimerFinished`)
      (if (>= (`self.Score`) (`self.ScoreLimit`))
        (`self.LevelCleared`)
        (else
          (`self.LevelFailed`))))))

(fn `StartTimer`
  (set `self.CountDown` true)
  (`self.TimerStarted`))

(fn `UserConstructionScript`)