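; BP_Forge is a forge actor that heats metal parts placed inside it.
; Overlap begin and end events add and remove BP_MetalParts actors from a CurrentlyHeating list.
; Each tick it raises the CurrentTemp of every valid listed part by HeatPerSecond scaled by delta time, with no upper limit applied here.
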(event `self.ReceiveActorBeginOverlap`
  (params (OtherActor :type "Actor Object Reference"))
  (bind _asbp_metal_parts (cast `/Game/Blueprints/BP_MetalParts` OtherActor))
  (`KismetArrayLibrary.Array_AddUnique` (`self.CurrentlyHeating`) _asbp_metal_parts))

(event `self.ReceiveActorEndOverlap`
  (params (OtherActor :type "Actor Object Reference"))
  (bind _asbp_metal_parts (cast `/Game/Blueprints/BP_MetalParts` OtherActor))
  (`KismetArrayLibrary.Array_RemoveItem` (`self.CurrentlyHeating`) _asbp_metal_parts))

(event `self.ReceiveTick`
  (params (DeltaSeconds :type "Float (single-precision)"))
  (for _array_element (`self.CurrentlyHeating`)
    (if (`KismetSystemLibrary.IsValid` _array_element)
      (set `/Game/Blueprints/BP_MetalParts.CurrentTemp` (+ (`/Game/Blueprints/BP_MetalParts.CurrentTemp` _array_element) (* DeltaSeconds (`self.HeatPerSecond`))) _array_element))))

(fn `UserConstructionScript`)