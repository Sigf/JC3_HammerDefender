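; BP_AssemblyBench is a crafting station that holds one wooden part and one metal part dropped onto it.
; On BeginPlay it binds to the ObjectCaught event of its child BP_CatcherObject.
; Each caught object is cast to BP_WoodPickable or BP_MetalParts; if that slot is empty, it is stored, its physics is disabled and its mesh snaps to the slot.
; No logic here combines or releases the parts.
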(event `self.ReceiveBeginPlay`
  (bind _asbp_catcher_object (cast `/Game/Blueprints/BaseClasses/BP_CatcherObject` (`ChildActorComponent.ChildActor` (`self.Catcher`))))
  (add `/Game/Blueprints/BaseClasses/BP_CatcherObject.ObjectCaught` _asbp_catcher_object (delegate `ObjectFound`)))

(event `ObjectFound`
  (params (Object :type "/Game/Blueprints/BaseClasses/BP_PickableObject Object Reference"))
  (bind _metalslot (`self.MetalSlot`))
  (bind _woodslot (`self.WoodSlot`))
  (`|ExecutionSequence`
    (:`then_0`
      (`/Engine/EditorBlueprintResources/StandardMacros.IsValid` (`self.CurrentWoodenPart`)
        (:`Is Not Valid`
          (bind _asbp_wood_pickable (cast `/Game/Blueprints/Props/BP_WoodPickable` Object))
          (bind _output_get (set `self.CurrentWoodenPart` _asbp_wood_pickable))
          (bind _staticmesh (`/Game/Blueprints/BaseClasses/BP_PickableStatic.StaticMesh` _output_get))
          (`PrimitiveComponent.SetSimulatePhysics` _staticmesh false)
          (`SceneComponent.K2_SetWorldTransform` _staticmesh (`KismetMathLibrary.MakeTransform` (`SceneComponent.K2_GetComponentLocation` _woodslot) (`SceneComponent.K2_GetComponentRotation` _woodslot)) false false))))
    (:`then_1`
      (`/Engine/EditorBlueprintResources/StandardMacros.IsValid` (`self.CurrentMetalPart`)
        (:`Is Not Valid`
          (bind _asbp_metal_parts (cast `/Game/Blueprints/BaseClasses/BP_MetalParts` Object))
          (bind _output_get_2 (set `self.CurrentMetalPart` _asbp_metal_parts))
          (bind _staticmesh_2 (`/Game/Blueprints/BaseClasses/BP_PickableStatic.StaticMesh` _output_get_2))
          (`PrimitiveComponent.SetSimulatePhysics` _staticmesh_2 false)
          (`SceneComponent.K2_SetWorldTransform` _staticmesh_2 (`KismetMathLibrary.MakeTransform` (`SceneComponent.K2_GetComponentLocation` _metalslot) (`SceneComponent.K2_GetComponentRotation` _metalslot)) false false))))))

(fn `UserConstructionScript`)