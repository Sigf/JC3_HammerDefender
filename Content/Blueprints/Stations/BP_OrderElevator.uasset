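; An order elevator station that shows customer orders on a board and accepts weapons to fill them.
; On BeginPlay it caches the BP_CustomerOrderUI widget from its OrderBoard component and creates a random order.
; When the ObjectFound event delivers a BP_Weapon, it asks the UI for a matching order and passes the result on to reduce that order's amount.
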(event `self.ReceiveBeginPlay`
  (`parent.ReceiveBeginPlay`)
  (bind _asbp_customer_order_ui (cast `/Game/Blueprints/UI/BP_CustomerOrderUI` (`WidgetComponent.GetUserWidgetObject` (`self.orderBoard`))))
  (bind _output_get (set `self.Order_UI` _asbp_customer_order_ui))
  (`/Game/Blueprints/UI/BP_CustomerOrderUI.CreateRandomOrder` _output_get))

(event `ObjectFound`
  (params (Object :type "/Game/Blueprints/BaseClasses/BP_PickableObject Object Reference"))
  (bind _asbp_weapon (cast `/Game/Blueprints/BaseClasses/BP_Weapon` Object))
  (bind _newparam (`/Game/Blueprints/UI/BP_CustomerOrderUI.HasOrderForWeapon` (stale `self.ReceiveBeginPlay` _output_get) _asbp_weapon))
  (`/Game/Blueprints/UI/BP_CustomerOrderUI.ReduceOrderAmount` (stale `self.ReceiveBeginPlay` _output_get) _newparam))

(fn `UserConstructionScript`
  (`parent.UserConstructionScript`))