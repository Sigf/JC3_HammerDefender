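; Woodworking bench station that turns caught wood into sword handles, axe handles or shield backs, with the selected product cycled through CycleOptions.
; Its child catcher reports each caught object, which increments the wood count and is then popped from the catcher.
; Tick pushes state to the widget and, while enough wood is stored, advances crafting.
; On completion it deducts wood and launches the spawned part with an impulse.
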(event `self.ReceiveBeginPlay`
  (bind _asbp_catcher_object (cast `/Game/Blueprints/BaseClasses/BP_CatcherObject` (`ChildActorComponent.ChildActor` (`self.WoodCatcher`))))
  (add `/Game/Blueprints/BaseClasses/BP_CatcherObject.ObjectCaught` _asbp_catcher_object (delegate `WoodAdded`)))

(event `WoodAdded`
  (params (Object :type "/Game/Blueprints/BaseClasses/BP_PickableObject Object Reference"))
  (`/Engine/EditorBlueprintResources/StandardMacros.IncrementInt` (`self.Wood Count`)
    (:`  `
      (bind _asbp_catcher_object (cast `/Game/Blueprints/BaseClasses/BP_CatcherObject` (`ChildActorComponent.ChildActor` (`self.WoodCatcher`))))
      (`/Game/Blueprints/BaseClasses/BP_CatcherObject.PopObject` _asbp_catcher_object))))

(event `self.ReceiveTick`
  (params (DeltaSeconds :type "Float (single-precision)"))
  (bind _currentlycrafting (`self.CurrentlyCrafting`))
  (`|ExecutionSequence`
    (:`then_0`
      (bind _asbp_woodworking_bench_ui (cast `/Game/Blueprints/UI/BP_WoodworkingBenchUI` (`WidgetComponent.GetUserWidgetObject` (`self.Widget`))))
      (set `/Game/Blueprints/UI/BP_WoodworkingBenchUI.CraftingStatus` (`self.Crafting Status`) _asbp_woodworking_bench_ui)
      (set `/Game/Blueprints/UI/BP_WoodworkingBenchUI.CurrentlyCrafting` _currentlycrafting _asbp_woodworking_bench_ui)
      (set `/Game/Blueprints/UI/BP_WoodworkingBenchUI.WoodCount` (`self.Wood Count`) _asbp_woodworking_bench_ui)
      (switch `/Game/Blueprints/E_WeaponComponent` _currentlycrafting
        (:`NewEnumerator1`
          (set `/Game/Blueprints/UI/BP_WoodworkingBenchUI.Required Wood` 1 _asbp_woodworking_bench_ui :!label _label))
        (:`NewEnumerator3`
          (goto _label))
        (:`NewEnumerator5`
          (set `/Game/Blueprints/UI/BP_WoodworkingBenchUI.Required Wood` 2 _asbp_woodworking_bench_ui))))
    (:`then_1`
      (bind _result (`self.CheckRecipe`))
      (if _result
        (bind _output_get (set `self.Crafting Status` (+ (`self.Crafting Status`) (/ DeltaSeconds (`self.Crafting Time`)))))
        (if (>= _output_get 1.0)
          (`self.PopObject`))))))

(fn `CheckRecipe`
  (returns (Result :type Boolean))
  (bind _wood_count (`self.Wood Count`))
  (switch `/Game/Blueprints/E_WeaponComponent` (`self.CurrentlyCrafting`)
    (:`NewEnumerator1`
      _)
    (:`NewEnumerator3`
      _)
    (:`NewEnumerator5`
      (return (>= _wood_count 2))))
  (return (>= _wood_count 1)))

(fn `CycleOptions`
  (bind _craftingoptions (`self.CraftingOptions`))
  (set `self.CurrentlyCrafting` (`|GetArrayItem` _craftingoptions (mod (+ (`KismetArrayLibrary.Array_Find` _craftingoptions (`self.CurrentlyCrafting`)) 1) (`KismetArrayLibrary.Array_Length` _craftingoptions)))))

(fn `PopObject`
  (locals (ClassToSpawn :type "/Game/Blueprints/BaseClasses/BP_WoodParts Class Reference"))
  (bind _wood_count (`self.Wood Count`))
  (bind _spawndirection (`self.SpawnDirection`))
  (switch `/Game/Blueprints/E_WeaponComponent` (`self.CurrentlyCrafting`)
    (:`NewEnumerator1`
      (set `local.ClassToSpawn` "/Game/Blueprints/WeaponsComponents/BP_SwordHandle.BP_SwordHandle_C")
      (set `self.Wood Count` (- _wood_count 1) :!label _label))
    (:`NewEnumerator3`
      (set `local.ClassToSpawn` "/Game/Blueprints/WeaponsComponents/BP_AxeHandle.BP_AxeHandle_C")
      (goto _label))
    (:`NewEnumerator5`
      (set `local.ClassToSpawn` "/Game/Blueprints/WeaponsComponents/BP_ShieldBack.BP_ShieldBack_C")
      (set `self.Wood Count` (- _wood_count 2))))
  (set `self.Crafting Status` 0.0)
  (bind _returnvalue (`|SpawnActorFromClass` (`local.ClassToSpawn`) (`KismetMathLibrary.MakeTransform` (`SceneComponent.K2_GetComponentLocation` _spawndirection) (`SceneComponent.K2_GetComponentRotation` _spawndirection)) "AlwaysSpawn" "OverrideRootScale" null null))
  (`PrimitiveComponent.AddImpulse` (`/Game/Blueprints/BaseClasses/BP_PickableStatic.StaticMesh` _returnvalue) (* (`SceneComponent.GetForwardVector` _spawndirection) (`self.SpawnStrength`)) "None" false))

(fn `ShowName`
  (returns (Name :type Text))
  (return (`|FormatText` "Woodworking Bench")))

(fn `UserConstructionScript`)