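; Anvil crafting station that holds one metal part and refines it under an animated hammer.
; A child catcher object reports caught metal parts, which are frozen and snapped to the slot until DropObject re-enables physics and pops them.
; Tick plays or stops the hammer animation based on whether a part is present and pushes its refinement to a status widget.
; CraftCurrentItem raises refinement in proportion to crafting speed and the part's temperature.
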(event `self.ReceiveBeginPlay`
  (bind _asbp_catcher_object (cast `/Game/Blueprints/BaseClasses/BP_CatcherObject` (`ChildActorComponent.ChildActor` (`self.Catcher`))))
  (add `/Game/Blueprints/BaseClasses/BP_CatcherObject.ObjectCaught` _asbp_catcher_object (delegate `ObjectFound`)))

(event `ObjectFound`
  (params (Object :type "/Game/Blueprints/BaseClasses/BP_PickableObject Object Reference"))
  (bind _metalpartslot (`self.MetalPartSlot`))
  (`/Engine/EditorBlueprintResources/StandardMacros.IsValid` (`self.CurrentMetalPart`)
    (:`Is Not Valid`
      (bind _asbp_metal_parts (cast `/Game/Blueprints/BaseClasses/BP_MetalParts` Object))
      (bind _output_get (set `self.CurrentMetalPart` _asbp_metal_parts))
      (bind _staticmesh (`/Game/Blueprints/BaseClasses/BP_PickableStatic.StaticMesh` _output_get))
      (`PrimitiveComponent.SetSimulatePhysics` _staticmesh false)
      (`SceneComponent.K2_SetWorldTransform` _staticmesh (`KismetMathLibrary.MakeTransform` (`SceneComponent.K2_GetComponentLocation` _metalpartslot) (`SceneComponent.K2_GetComponentRotation` _metalpartslot) (`SceneComponent.RelativeScale3D` _staticmesh)) false false))))

(event `self.ReceiveTick`
  (params (DeltaSeconds :type "Float (single-precision)"))
  (`|ExecutionSequence`
    (:`then_0`
      ;[1 1 1] Updates Hammer Animation
      (if (`self.AnimationStopped`)
        (`/Engine/EditorBlueprintResources/StandardMacros.IsValid` (`self.CurrentMetalPart`)
          (:`Is Valid`
            (`self.StartHammerAnimation`)))
        (else
          (`/Engine/EditorBlueprintResources/StandardMacros.IsValid` (`self.CurrentMetalPart`)
            (:`Is Not Valid`
              (`self.StopHammerAnimation`))))))
    (:`then_1`
      ;[1 1 1] Update Widget
      (bind _widget (`self.GetStatusWidget`))
      (`/Engine/EditorBlueprintResources/StandardMacros.IsValid` (`self.CurrentMetalPart`)
        (:`Is Valid`
          (set `/Game/Blueprints/UI/BP_AnvilStatus.CraftingStatus` (`/Game/Blueprints/BaseClasses/BP_MetalParts.RefinementState` (`self.CurrentMetalPart`)) _widget))
        (:`Is Not Valid`
          (set `/Game/Blueprints/UI/BP_AnvilStatus.CraftingStatus` 0.0 _widget))))))

(fn `CraftCurrentItem`
  (bind _currentmetalpart (`self.CurrentMetalPart`))
  (`/Engine/EditorBlueprintResources/StandardMacros.IsValid` _currentmetalpart
    (:`Is Valid`
      (set `/Game/Blueprints/BaseClasses/BP_MetalParts.RefinementState` (`KismetMathLibrary.FClamp` (+ (`/Game/Blueprints/BaseClasses/BP_MetalParts.RefinementState` _currentmetalpart) (* (`self.CraftingSpeed`) (`/Game/Blueprints/BaseClasses/BP_MetalParts.CurrentTemp` _currentmetalpart)))) _currentmetalpart))))

(fn `DropObject`
  (`PrimitiveComponent.SetSimulatePhysics` (`/Game/Blueprints/BaseClasses/BP_PickableStatic.StaticMesh` (`self.CurrentMetalPart`)) true)
  (set `self.CurrentMetalPart` null)
  (bind _asbp_catcher_object (cast `/Game/Blueprints/BaseClasses/BP_CatcherObject` (`ChildActorComponent.ChildActor` (`self.Catcher`))))
  (`/Game/Blueprints/BaseClasses/BP_CatcherObject.PopObject` _asbp_catcher_object))

(fn `GetStatusWidget`
  (returns (Widget :type "/Game/Blueprints/UI/BP_AnvilStatus Object Reference"))
  (bind _asbp_anvil_status (cast `/Game/Blueprints/UI/BP_AnvilStatus` (`WidgetComponent.GetUserWidgetObject` (`self.StatusWidget`))))
  (return _asbp_anvil_status))

(fn `StartHammerAnimation`
  (bind _skeletalmesh (`self.SkeletalMesh`))
  (`SkeletalMeshComponent.SetPosition` _skeletalmesh 0.0 true)
  (`SkeletalMeshComponent.SetPlayRate` _skeletalmesh 1.0)
  (set `self.AnimationStopped` false))

(fn `StopHammerAnimation`
  (bind _skeletalmesh (`self.SkeletalMesh`))
  (`SkeletalMeshComponent.SetPosition` _skeletalmesh 0.0 true)
  (`SkeletalMeshComponent.SetPlayRate` _skeletalmesh 0.0)
  (set `self.AnimationStopped` true))

(fn `UserConstructionScript`)