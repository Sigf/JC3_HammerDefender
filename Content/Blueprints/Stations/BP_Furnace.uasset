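; Furnace crafting station that turns caught iron into sword blades, axe blades or shield handles, with the selected component cycled on demand.
; Child-actor catchers feed iron count and coal heat, which decays each Tick and drives a coal material, light and status widget.
; Crafting progress scales with heat and needs enough iron, two for sword blades.
; Finished parts spawn hot and are launched by a physics impulse.
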(event `self.ReceiveBeginPlay`
  (`|ExecutionSequence`
    (:`then_0`
      (bind _returnvalue (`KismetMaterialLibrary.CreateDynamicMaterialInstance` "/Game/Materials/MAT_HotCoals_Inst.MAT_HotCoals_Inst"))
      (bind _output_get (set `self.CoalMaterial` _returnvalue))
      (`PrimitiveComponent.SetMaterial` (`self.Coals`) 0 _output_get))
    (:`then_1`
      (bind _asbp_catcher_object (cast `/Game/Blueprints/BaseClasses/BP_CatcherObject` (`ChildActorComponent.ChildActor` (`self.CoalCatcher`))))
      (add `/Game/Blueprints/BaseClasses/BP_CatcherObject.ObjectCaught` _asbp_catcher_object (delegate `CoalCaught`)))
    (:`then_2`
      (bind _asbp_catcher_object_2 (cast `/Game/Blueprints/BaseClasses/BP_CatcherObject` (`ChildActorComponent.ChildActor` (`self.IronCatcher`))))
      (add `/Game/Blueprints/BaseClasses/BP_CatcherObject.ObjectCaught` _asbp_catcher_object_2 (delegate `IronCaught`)))))

(event `CoalCaught`
  (params (Object :type "/Game/Blueprints/BaseClasses/BP_PickableObject Object Reference"))
  (set `self.CurrentCoalTemp` (`KismetMathLibrary.FClamp` (+ (`self.CurrentCoalTemp`) (`self.CoalFuelTemp`))))
  (bind _asbp_catcher_object (cast `/Game/Blueprints/BaseClasses/BP_CatcherObject` (`ChildActorComponent.ChildActor` (`self.CoalCatcher`))))
  (`/Game/Blueprints/BaseClasses/BP_CatcherObject.PopObject` _asbp_catcher_object))

(event `IronCaught`
  (params (Object :type "/Game/Blueprints/BaseClasses/BP_PickableObject Object Reference"))
  (`/Engine/EditorBlueprintResources/StandardMacros.IncrementInt` (`self.CurrentIronCount`)
    (:`  `
      (bind _asbp_catcher_object (cast `/Game/Blueprints/BaseClasses/BP_CatcherObject` (`ChildActorComponent.ChildActor` (`self.IronCatcher`))))
      (`/Game/Blueprints/BaseClasses/BP_CatcherObject.PopObject` _asbp_catcher_object))))

(event `self.ReceiveTick`
  (params (DeltaSeconds :type "Float (single-precision)"))
  (bind _currentironcount (`self.CurrentIronCount`))
  (bind _returnvalue (+ (`self.CraftingStatus`) (* (`self.CraftingSpeed`) DeltaSeconds (`self.CurrentCoalTemp`))))
  (`|ExecutionSequence`
    (:`then_0`
      ;[1 1 1] Check for Iron Status Update
      (bind _widget (`self.GetStatusWidget`))
      (set `/Game/Blueprints/UI/BP_FurnaceStatus.CurrentIronCount` (`self.CurrentIronCount`) _widget))
    (:`then_1`
      ;[1 1 1] Check for Coal Status Update
      (bind _output_get (set `self.CurrentCoalTemp` (`KismetMathLibrary.FClamp` (- (`self.CurrentCoalTemp`) (* (`self.TempDepletionRate`) DeltaSeconds)))))
      (`self.setCoalTemp` _output_get))
    (:`then_2`
      ;[1 1 1] Update Crafting
      (if (`|EnumEquality` (`self.CurrentComponent`) "NewEnumerator0")
        (if (> _currentironcount 1)
          (if (>= _returnvalue 1.0) :!label _label
            (`self.ItemCrafted_Event`)
            (set `self.CraftingStatus` 0.0)
            (else
              (set `self.CraftingStatus` _returnvalue)))
          (bind _widget_2 (`self.GetStatusWidget`))
          (set `/Game/Blueprints/UI/BP_FurnaceStatus.CurrentCraftingStatus` (`self.CraftingStatus`) _widget_2))
        (elif (> _currentironcount 0)
          (goto _label))))
    (:`then_3`
      (bind _widget_3 (`self.GetStatusWidget`))
      (set `/Game/Blueprints/UI/BP_FurnaceStatus.CraftingItemType` (`self.CurrentComponent`) _widget_3))))

(event `ItemCrafted_Event`
  (bind _currentironcount (`self.CurrentIronCount`))
  (bind _asbp_catcher_object (cast `/Game/Blueprints/BaseClasses/BP_CatcherObject` (`ChildActorComponent.ChildActor` (`self.IronCatcher`))))
  (`/Engine/EditorBlueprintResources/StandardMacros.DecrementInt` _currentironcount
    (:`  `
      (`/Game/Blueprints/BaseClasses/BP_CatcherObject.PopObject` _asbp_catcher_object)
      (if (`|EnumEquality` (`self.CurrentComponent`) "NewEnumerator0")
        (`/Game/Blueprints/BaseClasses/BP_CatcherObject.PopObject` _asbp_catcher_object)
        (`/Engine/EditorBlueprintResources/StandardMacros.DecrementInt` _currentironcount
          (:`  `
            _)))
      (`self.SpawnCraftedObject`))))

(fn `CircleCraftableObjects`
  (bind _craftablecomponents (`self.CraftableComponents`))
  (set `self.CraftingStatus` 0.0)
  (bind _result (`/Engine/EditorBlueprintResources/StandardMacros.IncrementInt` (`self.CurrentItemIndex`))
    (:`  `
      (if (>= _result (`KismetArrayLibrary.Array_Length` _craftablecomponents))
        (bind _output_get (set `self.CurrentItemIndex` 0))
        (set `self.CurrentComponent` (`|GetArrayItem` _craftablecomponents _output_get))
        (else
          (set `self.CurrentComponent` (`|GetArrayItem` _craftablecomponents _result)))))))

(fn `GetStatusWidget`
  (returns (Widget :type "/Game/Blueprints/UI/BP_FurnaceStatus Object Reference"))
  (bind _asbp_furnace_status (cast `/Game/Blueprints/UI/BP_FurnaceStatus` (`WidgetComponent.GetUserWidgetObject` (`self.CoalStatus`))))
  (return _asbp_furnace_status))

(fn `setCoalTemp`
  (params (Temp :type "Float (double-precision)"))
  (`MaterialInstanceDynamic.SetScalarParameterValue` (`self.CoalMaterial`) "Temperature" Temp)
  (`LightComponent.SetIntensity` (`self.CoalsLight`) (`KismetMathLibrary.Lerp` 0.0 (`self.MaxLightIntensity`) Temp))
  (bind _widget (`self.GetStatusWidget`))
  (set `/Game/Blueprints/UI/BP_FurnaceStatus.CurrentCoalTemp` Temp _widget))

(fn `ShowName`
  (returns (Name :type Text))
  (return (`|FormatText` "Furnace")))

(fn `SpawnCraftedObject`
  (switch `/Game/Blueprints/E_WeaponComponent` (`self.CurrentComponent`)
    (:`NewEnumerator0`
      (`self.SpawnObject` "/Game/Blueprints/WeaponsComponents/BP_SwordBlade.BP_SwordBlade_C"))
    (:`NewEnumerator2`
      (`self.SpawnObject` "/Game/Blueprints/WeaponsComponents/BP_AxeBlade.BP_AxeBlade_C"))
    (:`NewEnumerator4`
      (`self.SpawnObject` "/Game/Blueprints/WeaponsComponents/BP_ShieldHandle.BP_ShieldHandle_C"))))

(fn `SpawnObject`
  (params (PickableClass :type "/Game/Blueprints/BaseClasses/BP_PickableObject Class Reference"))
  (bind _spawndirection (`self.SpawnDirection`))
  (bind _returnvalue (`|SpawnActorFromClass` PickableClass (`SceneComponent.K2_GetComponentToWorld` _spawndirection) "AlwaysSpawn" "OverrideRootScale" null null))
  (bind _asbp_pickable_static (cast `/Game/Blueprints/BaseClasses/BP_PickableStatic` _returnvalue))
  (bind _staticmesh (`/Game/Blueprints/BaseClasses/BP_PickableStatic.StaticMesh` _asbp_pickable_static))
  (`PrimitiveComponent.WakeRigidBody` _staticmesh "None")
  (`PrimitiveComponent.AddImpulse` _staticmesh (* (`SceneComponent.GetForwardVector` _spawndirection) (`self.SpawnStrength`)) "None" false)
  (bind _asbp_metal_parts (cast `/Game/Blueprints/BaseClasses/BP_MetalParts` _asbp_pickable_static))
  (set `/Game/Blueprints/BaseClasses/BP_MetalParts.CurrentTemp` 1.0 _asbp_metal_parts))

(fn `UserConstructionScript`)