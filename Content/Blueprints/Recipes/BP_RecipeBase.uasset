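; BP_RecipeBase is a recipe base Blueprint whose MatchRecipe function tests input parts against a part list to yield a weapon type.
; It resets a counter, checks an input's class against PartList, and sets FoundMatch once the count reaches the list length, returning ResultingThing.
; Every branch returns inside the loop, so only the first input is evaluated, and FoundMatch is never cleared here.
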(fn `MatchRecipe`
  (params (InputParts :type "Array of /Game/Blueprints/BaseClasses/BP_PickableObject Object Reference (by ref)"))
  (returns (OutputWeaponType :type "/Game/Blueprints/BaseClasses/BP_PickableObject Class Reference") (match :type Boolean))
  (locals (foundMatch :type Boolean))
  (bind _partlist (`self.PartList`))
  (bind _output_get (set `self.PartMatchCount` 0)) ; ResetPartMatch
  (for _array_element InputParts
    (if (`KismetArrayLibrary.Array_Contains` _partlist (`GameplayStatics.GetObjectClass` _array_element))
      (bind _result (`/Engine/EditorBlueprintResources/StandardMacros.IncrementInt` _output_get)
        (:`  `
          (if (<= (`KismetArrayLibrary.Array_Length` _partlist) _result)
            (bind _output_get_2 (set `local.foundMatch` true))
            (return (`self.ResultingThing`) _output_get_2)
            (else
              _)))))
    (return null (`local.foundMatch`))))