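; BP_PickableStatic is a base class for pickable world objects represented by a static mesh.
; Its construction script applies the Mesh variable to the StaticMesh component.
; On BeginPlay it runs the parent logic, enables physics simulation on that component and sets it to ignore the Pawn collision channel.
; No pickup logic appears in this Blueprint itself.
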(event `self.ReceiveBeginPlay`
  (bind _staticmesh (`self.StaticMesh`))
  (`parent.ReceiveBeginPlay`)
  (`PrimitiveComponent.SetSimulatePhysics` _staticmesh true)
  (`PrimitiveComponent.SetCollisionResponseToChannel` _staticmesh "ECC_Pawn" "ECR_Ignore"))

(fn `UserConstructionScript`
  (`parent.UserConstructionScript`)
  (`StaticMeshComponent.SetStaticMesh` (`self.StaticMesh`) (`self.Mesh`)))